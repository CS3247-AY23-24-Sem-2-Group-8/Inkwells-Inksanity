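; Game mode for turn-based battles that sets up the fight, queues unit turns and can show the main menu.
; On BeginPlay it points the view at the front camera, gathers player and enemy units and registers them with the controller's battle HUD.
; Turn requests join a unique first-in queue, where a DoOnce gate starts one unit's ScrabbleCombatComponent turn until StartNextPlayerTurn resets it for the next.
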(event Custom|TurnRequest
  (params (Unit :type BP%20Unit%20Base%20Object%20Reference))
  ;[1 1 1] Turn Manager
  (Utilities|Array|AddUnique (Variables|Default|GetTurnOrder) Unit)
  (CallFunction|AttemptStartTurn) ; Requests to start its turn
)

(event Custom|AttemptStart%20Turn
  (bind _turnorder (Variables|Default|GetTurnOrder))
  (bind _output (Utilities|Array|Get(acopy) _turnorder))
  (bind _scrabblecombatcomponent (Variables|/Game/BP_UnitBase.BP_UnitBase_C|GetScrabbleCombatComponent _output))
  ;[1 1 1] Turn Manager
  (Utilities|FlowControl|DoOnce false
    (:Completed
      (if (Utilities|Array|IsValidIndex (Variables|Default|GetTurnOrder))
        (Default|StartUnitTurn _scrabblecombatcomponent)
        (EventDispatchers|BindEventtoTurnEnded _scrabblecombatcomponent (EventDispatchers|CreateEvent :!event Custom|StartNextPlayerTurn))
        (Utilities|Array|RemoveIndex (Variables|Default|GetTurnOrder))
        (else
          (CallFunction|StartNextPlayerTurn))))))

(event Custom|StartNextPlayerTurn
  (bind _turnorder (Variables|Default|GetTurnOrder))
  (bind _output (Utilities|Array|Get(acopy) _turnorder))
  (bind _scrabblecombatcomponent (Variables|/Game/BP_UnitBase.BP_UnitBase_C|GetScrabbleCombatComponent _output))
  ;[1 1 1] Turn Manager
  (Utilities|FlowControl|Sequence
    (:then_0
      (Utilities|FlowControl|DoOnce false) ; enters at Reset
    )
    (:then_1
      (if (Utilities|Array|IsValidIndex (Variables|Default|GetTurnOrder)) ; Start next player's turn if there is someone waiting
        (CallFunction|AttemptStartTurn)))))

(event Custom|ShowMainMenu
  (bind _returnvalue (Game|GetPlayerController 0))
  (bind _returnvalue_2 (UserInterface|CreateWidget "/Game/Widget/BP_MainMenuWidget.BP_MainMenuWidget_C" (Game|GetPlayerController 0)))
  (bind _output_get (Variables|Widgets|SetMainMenuWidget _returnvalue_2))
  (UserInterface|Viewport|AddtoViewport _output_get 0)
  (Input|SetInputModeUIOnly _returnvalue (Variables|Widgets|GetMainMenuWidget) "DoNotLock" false)
  (Variables|/Script/Engine.PlayerController|SetbShowMouseCursor _returnvalue true))

(event EventBeginPlay
  (CallFunction|StartGame))

(fn ConstructionScript)

(fn StartGame
  (bind _returnvalue (Actor|GetActorOfClass "/Game/BP_Camera_Front.BP_Camera_Front_C"))
  (bind _output_get (Variables|Default|SetMainCamera _returnvalue))
  (Game|Player|SetViewTargetwithBlend (Game|GetPlayerController 0) _output_get 0.0 "VTBlend_Linear" 0.0 false)
  (bind _outactors (Actor|GetAllActorsOfClass "/Game/BP_PlayerUnitBase.BP_PlayerUnitBase_C"))
  (Variables|Default|SetFriendlyUnits _outactors)
  (bind _outactors_2 (Actor|GetAllActorsOfClass "/Game/BP_EnemyUnitBase.BP_EnemyUnitBase_C"))
  (Variables|Default|SetEnemyUnits _outactors_2)
  (bind _asbp_turn_based_player_controller (Utilities|Casting|CastToBP_TurnBasedPlayerController (Game|GetPlayerController 0)))
  (bind _battle_hud (Variables|/Game/BP_TurnBasedPlayerController.BP_TurnBasedPlayerController_C|GetBattle%20HUD _asbp_turn_based_player_controller)
    (:then
      (Variables|Default|SetBattle%20HUD _battle_hud)
      (Utilities|FlowControl|Sequence
        (:then_0
          (for _array_element (Variables|Default|GetFriendlyUnits)
            (Default|AddFriendlyUnittoHUD (Variables|Default|GetBattle%20HUD) _array_element)))
        (:then_1
          (for _array_element_2 (Variables|Default|GetEnemyUnits)
            (Default|AddEnemyUnittoHUD (Variables|Default|GetBattle%20HUD) _array_element_2)))))
    (:else)))