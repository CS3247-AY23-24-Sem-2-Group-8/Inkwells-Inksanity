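; Grid board actor for a turn-based letter-tile word game, usable by the player or an AI opponent.
; Fills a flat array with tiles drawn randomly from a bag; removed tiles feed a used pile that replenishes it, while columns collapse and refill.
; Selected tiles line up at an arrow.
; For AI, tiles start hidden; BP_ScrabbleEnemyAI builds letters iteratively, then Play randomly picks among dictionary-valid words and reveals its tiles.
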(event EventBeginPlay
  (if (Math|Boolean|ANDBoolean (>= (Utilities|Array|Length (Variables|Default|GetBag)) (* (Variables|Default|GetRows) (Variables|Default|GetColumns))) (> (Variables|Default|GetRows) 0) (> (Variables|Default|GetColumns) 0))
    (if (Variables|Default|GetIs%20AI)
      (bind _asbp_turn_based_game_mode (Utilities|Casting|CastToBP_TurnBasedGameMode (Game|GetGameMode)))
      (Variables|Default|SetDictionary (Variables|/Game/BP_TurnBasedGameMode.BP_TurnBasedGameMode_C|GetDictionary _asbp_turn_based_game_mode))
      (bind _returnvalue (Game|ConstructObjectfromClass "/Game/BP_ScrabbleEnemyAI.BP_ScrabbleEnemyAI_C"))
      (bind _output_get (Variables|Default|SetAI _returnvalue))
      (Class|ScrabbleEnemyAI|InitialiseAI _output_get 0.0 (Variables|Default|GetDictionary) 0.1)
      (Rendering|SetVisibility (Variables|Default|GetDefaultSceneRoot) false true))
    (CallFunction|InitialiseGrid)))

(fn ConstructionScript)

(fn GetWorldLocation
  (params (Board%20Address :type Integer))
  (bind _columns (Variables|Default|GetColumns))
  (bind _tile_size (Variables|Default|GetTile%20Size))
  (return (+ (+ (Transformation|GetActorLocation) (Math|Vector|MakeVector (* (* (- (Variables|Default|GetColumns) 1) -0.5) (.x (Variables|Default|GetTile%20Size))) 1.0 (* (* (- (Variables|Default|GetRows) 1) 0.5) (.y (Variables|Default|GetTile%20Size))))) (Math|Vector|MakeVector (* (Math|Integer|%(Integer) Board%20Address _columns) (.x _tile_size)) 0.0 (* (.y _tile_size) (/ Board%20Address _columns) -1.0)))))

(fn GetTile
  (params (Board%20Address :type Integer))
  (if (Utilities|Array|IsValidIndex (Variables|Default|GetBoard) Board%20Address)
    (return (Utilities|Array|Get(acopy) (Variables|Default|GetBoard) Board%20Address))))

(fn GetTranslatedBoardAddress
  (params (Reference%20Board%20Address :type Integer) (Row%20Offset :type Integer) (Col%20Offset :type Integer))
  (bind _columns (Variables|Default|GetColumns))
  (bind _columns_2 (Variables|Default|GetColumns))
  (bind _returnvalue (Math|Integer|%(Integer) Reference%20Board%20Address _columns))
  (bind _returnvalue_2 (/ Reference%20Board%20Address _columns_2))
  (bind _returnvalue_3 (+ _returnvalue Col%20Offset))
  (bind _returnvalue_4 (+ _returnvalue_2 Row%20Offset))
  (if (and (== _returnvalue_3 (Math|Integer|Clamp(Integer) _returnvalue_3 0 (- (Variables|Default|GetColumns) 1))) (== _returnvalue_4 (Math|Integer|Clamp(Integer) _returnvalue_4 0 (- (Variables|Default|GetRows) 1))))
    (return (+ Reference%20Board%20Address Col%20Offset (* Row%20Offset (Variables|Default|GetColumns))) true)
    (else
      (return -1 false))))

(fn RemoveSelectedTiles
  (for _array_element (Variables|Default|GetSelected%20Tiles)
    ;[1 1 1] Remove all reference of the tile and destroy it. Move the data into the used tile array.
    (Utilities|Array|Add (Variables|Default|GetUsed%20Tiles) (Variables|/Game/BP_Tile.BP_Tile_C|GetTile%20Data _array_element))
    (CallFunction|RemoveTilefromBoard (Variables|/Game/BP_Tile.BP_Tile_C|GetBoard%20Address _array_element))
    (Actor|DestroyActor _array_element))
  (Utilities|Array|Clear (Variables|Default|GetSelected%20Tiles))
  (CallFunction|MoveTilesDown))

(fn GetSelectedTiles'Data
  (for _array_element (Variables|Default|GetSelected%20Tiles)
    (Utilities|Array|Add (LocalVariables|GetTile%20Datas) (Variables|/Game/BP_Tile.BP_Tile_C|GetTile%20Data _array_element)))
  (return (LocalVariables|GetTile%20Datas)))

(fn OnTileSelected
  (params (Selected%20Tile :type BP%20Tile%20Object%20Reference))
  (Utilities|Array|Add (Variables|Default|GetSelected%20Tiles) Selected%20Tile)
  (CallFunction|UpdateSelectedTilePlacements)
  (Default|CallBoardStateChanged)
  (if (Variables|Default|GetIs%20AI)
    (Rendering|SetActorHiddenInGame Selected%20Tile false)))

(fn OnTileUnselected
  (params (Tile :type BP%20Tile%20Object%20Reference))
  (Utilities|Array|RemoveItem (Variables|Default|GetSelected%20Tiles) Tile)
  (CallFunction|UpdateSelectedTilePlacements)
  (bind _location (CallFunction|GetWorldLocation (Variables|/Game/BP_Tile.BP_Tile_C|GetBoard%20Address Tile)))
  (Default|SetExpectedLocation Tile _location)
  (Default|CallBoardStateChanged))

(fn OnTileFinishedFalling
  (params (Tile :type BP%20Tile%20Object%20Reference))
  (Utilities|Array|RemoveItem (Variables|Default|GetFalling%20Tiles) Tile)
  (if (== (Utilities|Array|Length (Variables|Default|GetFalling%20Tiles)) 0)
    (CallFunction|RefillBoard)))

(fn RemoveTilefromBoard
  (params (Board%20Address :type Integer))
  (if (Utilities|Array|IsValidIndex (Variables|Default|GetBoard) Board%20Address)
    (Utilities|Array|SetArrayElem (Variables|Default|GetBoard) Board%20Address 0)))

(fn RetrieveRandomTilefromBag
  (bind _output_get (LocalVariables|SetTarget%20Index (.OutIndex (Utilities|Array|Random (Variables|Default|GetBag))) :!label _label)) ; IMPORTANT! Must set variable here and always reference this variable. Else it will constantly generate a new random index
  (if (>= _output_get 0)
    ;[1 1 1] Retrieve and remove the tile from the bag
    (LocalVariables|SetRetrieved%20Tile (Utilities|Array|Get(acopy) (Variables|Default|GetBag) (LocalVariables|GetTarget%20Index)))
    (Utilities|Array|RemoveIndex (Variables|Default|GetBag) (LocalVariables|GetTarget%20Index))
    (return (LocalVariables|GetRetrieved%20Tile))
    (else
      (Utilities|FlowControl|Sequence
        (:then_0
          ;[1 1 1] Refills bag with the used tiles if bag is empty
          (for _array_element (Variables|Default|GetUsed%20Tiles)
            (Utilities|Array|Add (Variables|Default|GetBag) _array_element))
          (Utilities|Array|Clear (Variables|Default|GetUsed%20Tiles)))
        (:then_1
          ;[1 1 1] Important. Only retry if the bag is not empty. To prevent infinite recursion
          (if (Utilities|Array|IsNotEmpty (Variables|Default|GetBag))
            (goto _label)))))))

(fn CreateTile
  (params (Row :type Integer%20%28by%20ref%29) (Col :type Integer%20%28by%20ref%29))
  (bind (_output_board_address _isvalid) (CallFunction|GetTranslatedBoardAddress 0 Row Col))
  (if _isvalid
    (bind _location (CallFunction|GetWorldLocation _output_board_address)) ; Get expected location here
    (bind _world_location (CallFunction|GetWorldLocationwithOffset _output_board_address (* Row -1))) ; Set its current location to be the top of the column
    (bind _tile_data (CallFunction|RetrieveRandomTilefromBag))
    (bind _returnvalue (Game|SpawnActorfromClass "/Game/BP_Tile.BP_Tile_C" (Math|Transform|MakeTransform _world_location) "AdjustIfPossibleButAlwaysSpawn" "MultiplyWithRoot" 0 _tile_data self _location 0))
    (Variables|/Game/BP_Tile.BP_Tile_C|SetBoard%20Address _returnvalue _output_board_address)
    (Utilities|Array|SetArrayElem (Variables|Default|GetBoard) _output_board_address _returnvalue)
    (if (Variables|Default|GetIs%20AI)
      (Rendering|SetActorHiddenInGame _returnvalue true)
      (Variables|/Game/BP_Tile.BP_Tile_C|SetIs%20Interactable _returnvalue false))))

(fn InitialiseGrid
  (Utilities|Array|Resize (Variables|Default|GetBoard) (* (Variables|Default|GetRows) (Variables|Default|GetColumns)))
  (for _index (range 0 (- (Variables|Default|GetColumns) 1))
    (for _index_2 (range 0 (- (Variables|Default|GetRows) 1))
      (CallFunction|CreateTile _index_2 _index))))

(fn RefillBoard
  (for _index (range 0 (- (Variables|Default|GetColumns) 1))
    (LocalVariables|SetCurrent%20Col _index)
    (bind _index_2 (Utilities|FlowControl|ForLoopwithBreak 0 (- (Variables|Default|GetRows) 1) :!label _label)
      (:LoopBody
        (bind _output_get (LocalVariables|SetCurrent%20Row _index_2))
        (bind _output_board_address (CallFunction|GetTranslatedBoardAddress 0 _output_get (LocalVariables|GetCurrent%20Col)))
        (bind _tile (CallFunction|GetTile _output_board_address))
        (Utilities|IsValid _tile ; Break when encounter a valid tile in column. Assumes that this function always runs after Move Tiles Down
          (:Is%20Valid
            (goto _label Break))
          (:Is%20Not%20Valid
            (CallFunction|CreateTile (LocalVariables|GetCurrent%20Row) (LocalVariables|GetCurrent%20Col))))))))

(fn MoveTilesDown
  ;[1 1 1] Find a tile in column that is empty
  (for _index (range 0 (- (Variables|Default|GetColumns) 0))
    (bind _index_2 (Utilities|FlowControl|ForLoopwithBreak 1 (Variables|Default|GetRows) :!label _label)
      (:LoopBody
        (bind (_output_board_address _isvalid) (CallFunction|GetTranslatedBoardAddress 0 (- (Variables|Default|GetRows) _index_2) _index))
        (if _isvalid
          (bind _tile (CallFunction|GetTile _output_board_address))
          (Utilities|IsValid _tile
            (:Is%20Not%20Valid
              ;[1 1 1] Get valid tile above the empty tile
              (LocalVariables|SetIs%20Broken false)
              (bind _index_3 (Utilities|FlowControl|ForLoopwithBreak 1 (- (Variables|Default|GetRows) _index_2) :!label _label_2)
                (:LoopBody
                  (bind (_output_board_address_2 _isvalid_2) (CallFunction|GetTranslatedBoardAddress _output_board_address (* _index_3 -1)))
                  (if _isvalid_2
                    (bind _tile_2 (CallFunction|GetTile _output_board_address_2))
                    (Utilities|IsValid _tile_2
                      (:Is%20Valid
                        ;[1 1 1] Move Tile to empty tile
                        (Utilities|Array|SetArrayElem (Variables|Default|GetBoard) _output_board_address_2 0)
                        (Utilities|Array|SetArrayElem (Variables|Default|GetBoard) _output_board_address _tile_2)
                        (bind _output_get (Variables|/Game/BP_Tile.BP_Tile_C|SetBoard%20Address _tile_2 _output_board_address))
                        (bind _location (CallFunction|GetWorldLocation _output_get))
                        (Default|SetExpectedLocation _tile_2 _location)
                        (Utilities|Array|Add (Variables|Default|GetFalling%20Tiles) _tile_2)
                        (LocalVariables|SetIs%20Broken true)
                        (goto _label_2 Break)))))
                (:Completed
                  ;[1 1 1] Break row loop when there are no more valid tiles
                  (if (not (LocalVariables|GetIs%20Broken))
                    (goto _label Break))))))))
      (:Completed
        ;[1 1 1] Immediately refill when no falling tiles to trigger the refill.
        (if (Utilities|Array|IsEmpty (Variables|Default|GetFalling%20Tiles))
          (CallFunction|RefillBoard))))))

(fn UpdateSelectedTilePlacements
  (for (_array_element _array_index) (Variables|Default|GetSelected%20Tiles)
    (bind _location (CallFunction|GetWorldLocationOfSelectedTile _array_index))
    (Default|SetExpectedLocation _array_element _location)))

(fn GetWorldLocationOfSelectedTile
  (params (Index :type Integer))
  (bind _tile_size (Variables|Default|GetTile%20Size))
  (return (+ (+ (Transformation|GetWorldLocation (Variables|Default|GetArrow)) (Math|Vector|MakeVector (* (/ (Utilities|Array|Length (Variables|Default|GetSelected%20Tiles)) -2) (.x _tile_size)) 5.0 0.0)) (* (Math|Vector|MakeVector (.x _tile_size) 0.0 0.0) (+ (Math|Conversions|ToFloat(Integer) Index) 0.5)))))

(fn GetWorldLocationwithOffset
  (params (Board%20Address :type Integer) (Row%20Offset :type Integer) (Col%20Offset :type Integer))
  (bind _output_board_address (CallFunction|GetTranslatedBoardAddress Board%20Address Row%20Offset Col%20Offset))
  (bind _location (CallFunction|GetWorldLocation _output_board_address))
  (return _location))

(fn ClearBoard
  (for _array_element (Variables|Default|GetBoard)
    ;[1 1 1] Remove all reference of the tile and destroy it. Move the data into the used tile array.
    (Utilities|Array|Add (Variables|Default|GetUsed%20Tiles) (Variables|/Game/BP_Tile.BP_Tile_C|GetTile%20Data _array_element))
    (Actor|DestroyActor _array_element))
  (Utilities|Array|Clear (Variables|Default|GetSelected%20Tiles))
  (CallFunction|RefillBoard))

(fn UnselectAll
  (bind _arrayelement (Utilities|Array|ReverseforEachLoop (Variables|Default|GetSelected%20Tiles))
    (:LoopBody
      (CallFunction|OnTileUnselected _arrayelement))))

(fn ScrambleBoard
  (CallFunction|UnselectAll)
  (Utilities|Array|Shuffle (Variables|Default|GetBoard))
  (for (_array_element _array_index) (Variables|Default|GetBoard)
    (bind _location (CallFunction|GetWorldLocation _array_index))
    (Default|SetExpectedLocation _array_element _location)
    (Variables|/Game/BP_Tile.BP_Tile_C|SetBoard%20Address _array_element _array_index)))

(fn Simulate
  (if (Variables|Default|GetIs%20AI)
    (bind _output_get (LocalVariables|SetTiles (Utilities|Array|MakeArray "")))
    (Utilities|Array|Clear _output_get)
    (for _array_element (Variables|Default|GetBoard)
      (Utilities|Array|Add (LocalVariables|GetTiles) (Utilities|Struct|MakeBoardTile (.letter (Variables|/Game/BP_Tile.BP_Tile_C|GetTile%20Data _array_element)) (.point (Variables|/Game/BP_Tile.BP_Tile_C|GetTile%20Data _array_element)))))
    (Class|ScrabbleEnemyAI|SetBoard (Variables|Default|GetAI) (LocalVariables|GetTiles))
    (CallFunction|GetNextAction)))

(fn GetNextAction
  (if (< (Variables|Default|GetIteration) 16)
    (bind _ai (Variables|Default|GetAI)
      (:then
        (EventDispatchers|BindEventtoOnFinishNextAction _ai (EventDispatchers|CreateEvent :!event OnFinishGetNextAction))
        (Class|ScrabbleEnemyAI|GetNextAction _ai))
      (:else))
    (else
      (Variables|Default|SetIteration 0))))

(fn OnFinishGetNextAction
  (params (Character :type String) (Point :type Integer))
  (bind _output_get (LocalVariables|SetCurrent%20Char Character))
  (bind _output_get_2 (LocalVariables|SetCurrent%20Point Point))
  (Development|PrintString _output_get)
  (if (Math|Boolean|NORBoolean (== _output_get_2 -1) (Utilities|Array|IsEmpty _output_get))
    (Utilities|Array|Add (Variables|Default|GetSelected%20Tile%20Data) (Utilities|Struct|MakeTileData (LocalVariables|GetCurrent%20Char) (LocalVariables|GetCurrent%20Point)))
    (bind _output_get_3 (Variables|Default|SetCurrent%20Word (Utilities|String|Append (Variables|Default|GetCurrent%20Word) (LocalVariables|GetCurrent%20Char))))
    (Development|PrintString _output_get_3)
    (if (Class|ScrabbleDictionary|IsValidWord (Variables|Default|GetDictionary) _output_get_3)
      (Development|PrintString "Word Found")
      (Utilities|Array|Add (Variables|Default|GetWord%20Indices) (Variables|Default|GetIteration)))
    (Variables|Default|SetIteration (+ (Variables|Default|GetIteration) 1))
    (CallFunction|GetNextAction)
    (else
      (Default|CallFinishedTurn))))

(fn SelectTileonBoard
  (params (Tile%20Data :type Tile%20Data%20Structure))
  (LocalVariables|SetCurrent%20Char (.letter Tile%20Data))
  (LocalVariables|SetCurrent%20Point (.point Tile%20Data))
  (bind _array_element (Utilities|Array|ForEachLoopwithBreak (Variables|Default|GetBoard) :!label _label)
    (:LoopBody
      (if (Math|Boolean|ANDBoolean (Utilities|Enum|Equal(Enum) (.letter (Variables|/Game/BP_Tile.BP_Tile_C|GetTile%20Data _array_element)) (LocalVariables|GetCurrent%20Char)) (== (.point (Variables|/Game/BP_Tile.BP_Tile_C|GetTile%20Data _array_element)) (LocalVariables|GetCurrent%20Point)) (not (Utilities|Array|ContainsItem (Variables|Default|GetSelected%20Tiles) _array_element)))
        (CallFunction|OnTileSelected _array_element)
        (goto _label Break)))))

(fn Play
  (bind _word_indices (Variables|Default|GetWord%20Indices))
  (bind (_array_element _array_index) (Utilities|Array|ForEachLoopwithBreak _word_indices :!label _label)
    (:LoopBody
      (LocalVariables|SetSelected%20Word _array_element)
      (if (< _array_index (- (Utilities|Array|Length _word_indices) 1))
        (if (not (<= (Math|Random|RandomFloatinRange 0.0 1.0) (Variables|Default|GetProbability%20of%20Selecting%20Longer%20Word)))
          (goto _label Break))
        (else
          (goto _label Break))))
    (:Completed
      (for _index (range 0 (LocalVariables|GetSelected%20Word))
        (Development|PrintString (.Letter (Utilities|Struct|BreakTileData (Utilities|Array|Get(acopy) (Variables|Default|GetSelected%20Tile%20Data) _index))))
        (CallFunction|SelectTileonBoard (Utilities|Array|Get(acopy) (Variables|Default|GetSelected%20Tile%20Data) _index)))
      (Utilities|Array|Clear (Variables|Default|GetSelected%20Tile%20Data))
      (Utilities|Array|Clear (Variables|Default|GetWord%20Indices))
      (Variables|Default|SetCurrent%20Word "")
      (Variables|Default|SetIteration 0)
      (Development|PrintString "end"))))