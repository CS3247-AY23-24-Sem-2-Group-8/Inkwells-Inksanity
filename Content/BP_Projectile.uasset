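; Projectile actor that flies to the location its Target had at BeginPlay, without homing on later movement.
; Each Tick steps a fixed distance toward that point, unscaled by delta time and without sweep, snapping onto it when the squared distance is small enough.
; Arrival triggers OnCollide, which hides the sphere, activates Niagara, then after a short delay calls OnCollision with Target and destroys the actor.
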(event Custom|On%20Collide
  (Rendering|SetVisibility (Variables|Default|GetSphere) false false)
  (Components|Activation|Activate (Variables|Default|GetNiagara) false)
  (Utilities|FlowControl|Delay 0.5)
  (Default|CallOnCollision (Variables|Default|GetTarget))
  (Actor|DestroyActor))

(event EventBeginPlay
  (Variables|Default|SetExpected%20Location (Transformation|GetActorLocation (Variables|Default|GetTarget))))

(event EventTick
  (params (DeltaSeconds :type Float%20%28single-precision%29))
  (CallFunction|MoveTick DeltaSeconds))

(fn ConstructionScript)

(fn MoveTick
  (params (Delta%20Time :type Float%20%28double-precision%29))
  (Transformation|SetActorLocation (+ (Transformation|GetActorLocation) (* (Math|Vector|Normalize (- (Variables|Default|GetExpected%20Location) (Transformation|GetActorLocation))) 10)) false false)
  (if (< (Class|KismetMathLibrary|VectorDistanceSquared (Transformation|GetActorLocation) (Variables|Default|GetExpected%20Location)) 1e+01)
    (Transformation|SetActorLocation (Variables|Default|GetExpected%20Location) false false)
    (CallFunction|OnCollide)))