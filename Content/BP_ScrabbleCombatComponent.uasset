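; Combat component that lets player and enemy units fight turn-based battles by spelling words on a Scrabble-style tile board.
; Each unit spawns a board from a data-table tile bag: players use an action menu, while AI boards sit off-screen and play themselves.
; Dictionary-valid words trigger a melee run, montage and tile-point damage.
; Timed requests to the game mode drive turns, which begin with a game-over check.
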(event Custom|Execute%20AI%20Attack
  (bind (_is_valid _selected_tile_data) (CallFunction|CheckValidity))
  (if _is_valid
    (Variables|Default|SetCurrent%20Tile%20Data _selected_tile_data)
    (bind _board (Variables|Default|GetBoard)
      (:then
        (Default|RemoveSelectedTiles _board)
        (bind _asbp_turn_based_game_mode (Utilities|Casting|CastToBP_TurnBasedGameMode (Game|GetGameMode)))
        (Development|PrintString "Hello")
        (CallFunction|MeleeAttack (Utilities|Array|Get(acopy) (Variables|/Game/BP_TurnBasedGameMode.BP_TurnBasedGameMode_C|GetFriendlyUnits _asbp_turn_based_game_mode))))
      (:else))
    (else
      (Utilities|FlowControl|Delay 1.0)
      (CallFunction|ClearBoard))))

(event Custom|Attack
  (if (Utilities|ClassIsChildOf (Utilities|GetClass (Variables|Default|GetUnit%20Character)) "/Game/BP_PlayerUnitBase.BP_PlayerUnitBase_C")
    (CallFunction|ExecutePlayerAttack)
    (else
      (CallFunction|ExecuteAIAttack))))

(event Custom|Melee%20Attack
  (params (Enemy%20Target :type BP%20Unit%20Base%20Object%20Reference))
  (bind _battle_position (Variables|Default|GetBattle%20Position))
  (bind (_location _rotation) (Math|Transform|BreakTransform _battle_position))
  (AI|AIMoveTo (Variables|Default|GetUnit%20Character) "0, 0, 0" Enemy%20Target 1e+02 false ; Move to enemy target
    (:then
      ;[1 1 1] Disable action menu when executing action
      (bind _action_menu (Variables|Default|GetAction%20Menu)
        (:then
          (Widget|SetRenderOpacity _action_menu 0.5)
          (Widget|SetIsEnabled _action_menu false))
        (:else)))
    (:OnSuccess
      (bind _attack_montage (Variables|Default|GetAttack%20Montage)
        (:then
          (Animation|Montage|PlayMontage (Variables|/Script/Engine.Character|GetMesh (Variables|Default|GetUnit%20Character)) _attack_montage ; Play Attack animation if set
            (:OnCompleted
              _)))
        (:else
          _))
      ;[1 1 1] Deal damage to enemy
      (bind (_damage _damage_type_class) (CallFunction|CalculateDamage (Variables|Default|GetCurrent%20Tile%20Data)))
      (Game|Damage|ApplyDamage Enemy%20Target _damage 0 (Variables|Default|GetUnit%20Character) _damage_type_class)
      (Utilities|Array|Clear (Variables|Default|GetCurrent%20Tile%20Data))
      ;[1 1 1] Move back to original position
      (AI|AIMoveTo (Variables|Default|GetUnit%20Character) _location 0 5.0 false
        (:OnSuccess
          (Transformation|SetActorRotation (Variables|Default|GetUnit%20Character) _rotation)
          (Utilities|FlowControl|Delay 1.0)
          (CallFunction|EndUnitTurn))))))

(event EventBeginPlay
  (bind _asbp_unit_base (Utilities|Casting|CastToBP_UnitBase (Components|GetOwner)))
  (bind _output_get (Variables|Default|SetUnit%20Character _asbp_unit_base))
  (Variables|Default|SetBattle%20Position (Transformation|GetActorTransform _output_get))
  (if (Utilities|ClassIsChildOf (Utilities|GetClass (Variables|Default|GetUnit%20Character)) "/Game/BP_PlayerUnitBase.BP_PlayerUnitBase_C")
    (bind _returnvalue (UserInterface|CreateWidget "/Game/Widget/BP_ActionMenu.BP_ActionMenu_C"))
    (bind _output_get_2 (Variables|Default|SetAction%20Menu _returnvalue))
    (UserInterface|Viewport|AddtoViewport _output_get_2 0)
    (CallFunction|CreateBoard false 0.0)
    (else
      (Utilities|FlowControl|Delay 0.2)
      (CallFunction|CreateBoard true (Variables|Default|GetProbability))))
  (CallFunction|BeginBattle))

(fn StartUnitTurn
  (bind (_isgameover _hasplayerwon) (CallFunction|CheckGameOver (Variables|Default|GetUnit%20Character)))
  (if _isgameover
    (if _hasplayerwon
      (Game|OpenLevel(byName) "WorldMap")
      (bind _asbp_game_instance (Utilities|Casting|CastToBP_GameInstance (Game|GetGameInstance)))
      (Variables|/Game/BP_GameInstance.BP_GameInstance_C|SetCurrent%20Player%20Health _asbp_game_instance (Variables|/Game/BP_UnitBase.BP_UnitBase_C|GetHealth_Current (Variables|Default|GetUnit%20Character)))
      (else
        (bind _returnvalue (UserInterface|CreateWidget "/Game/Widget/BP_GameOverWidget.BP_GameOverWidget_C" (Game|GetPlayerController 0)))
        (Default|RenderMenuText _returnvalue _hasplayerwon)
        (bind _output_get (Variables|Default|SetGameOverScreen _returnvalue))
        (Input|SetInputModeUIOnly (Game|GetPlayerController 0) _output_get "DoNotLock" false)
        (UserInterface|Viewport|AddtoViewport (Variables|Default|GetGameOverScreen) 0)))
    (else
      (Development|PrintText (Variables|/Game/BP_UnitBase.BP_UnitBase_C|GetName (Variables|Default|GetUnit%20Character)))
      (if (Utilities|ClassIsChildOf (Utilities|GetClass (Variables|Default|GetUnit%20Character)) "/Game/BP_PlayerUnitBase.BP_PlayerUnitBase_C")
        (bind _action_menu (Variables|Default|GetAction%20Menu)
          (:then
            (Widget|SetRenderOpacity _action_menu 1.0)
            (Widget|SetIsEnabled _action_menu true)
            (EventDispatchers|BindEventtoCommandAttack _action_menu (EventDispatchers|CreateEvent :!event Custom|Attack))
            (EventDispatchers|BindEventtoCommandClear _action_menu (EventDispatchers|CreateEvent :!event ClearBoard))
            (EventDispatchers|BindEventtoCommandUnselect _action_menu (EventDispatchers|CreateEvent :!event UnselectTiles))
            (EventDispatchers|BindEventtoCommandScramble _action_menu (EventDispatchers|CreateEvent :!event Scramble)))
          (:else))
        (else
          (CallFunction|Attack))))))

(fn EndUnitTurn
  (Default|CallTurnEnded)
  (bind _asbp_player_unit_base (Utilities|Casting|CastToBP_PlayerUnitBase (Variables|Default|GetUnit%20Character))
    (:then
      (bind _asbp_game_instance (Utilities|Casting|CastToBP_GameInstance (Game|GetGameInstance)))
      (Variables|/Game/BP_GameInstance.BP_GameInstance_C|SetCurrent%20Player%20Health _asbp_game_instance (Variables|/Game/BP_UnitBase.BP_UnitBase_C|GetHealth_Current _asbp_player_unit_base))
      (CallFunction|BeginBattle))
    (:CastFailed
      (CallFunction|BeginBattle))))

(fn BeginBattle
  (Utilities|Time|SetTimerbyFunctionName 0 "RequestTurn" (Variables|Default|GetTime%20Between%20Turns)))

(fn RequestTurn
  (if (Utilities|ClassIsChildOf (Utilities|GetClass (Variables|Default|GetUnit%20Character)) "/Game/BP_EnemyUnitBase.BP_EnemyUnitBase_C")
    (bind _board (Variables|Default|GetBoard)
      (:then
        (Default|Play _board))
      (:else)))
  (bind _asbp_turn_based_game_mode (Utilities|Casting|CastToBP_TurnBasedGameMode (Game|GetGameMode)))
  (Default|TurnRequest _asbp_turn_based_game_mode (Variables|Default|GetUnit%20Character)))

(fn CalculateDamage
  (params (Tile%20Data :type Array%20of%20Tile%20Data%20Structures))
  (if (Utilities|Array|IsEmpty Tile%20Data)
    (LocalVariables|SetCurrent%20Damage 8.0)
    (else
      (for _array_element Tile%20Data
        (LocalVariables|SetCurrent%20Damage (+ (LocalVariables|GetCurrent%20Damage) (.point _array_element))))))
  (return (LocalVariables|GetCurrent%20Damage) (Variables|Default|GetDefault%20Damage%20Type%20Class)))

(fn CheckifWordIsValid
  (params (Word :type String))
  (bind _asbp_turn_based_game_mode (Utilities|Casting|CastToBP_TurnBasedGameMode (Game|GetGameMode))
    (:then
      (return (Class|ScrabbleDictionary|IsValidWord (Variables|/Game/BP_TurnBasedGameMode.BP_TurnBasedGameMode_C|GetDictionary _asbp_turn_based_game_mode) Word)))
    (:CastFailed
      (return false))))

(fn CreateBoard
  (params (Is%20AI :type Boolean) (Probability :type Float%20%28double-precision%29))
  (bind _outrownames (DataTable|GetDataTableRowNames "/Game/Bag.Bag"))
  (for _array_element _outrownames
    (bind _returnvalue (Utilities|GetDataTableRow "/Game/Bag.Bag" _array_element)
      (:then
        (for _index (range 0 (- (.Quantity (Utilities|Struct|BreakTileQuantity _returnvalue)) 1))
          (Utilities|Array|Add (LocalVariables|GetBag) (.Tile (Utilities|Struct|BreakTileQuantity _returnvalue)))))))
  (if Is%20AI
    (bind _returnvalue_2 (Game|SpawnActorfromClass "/Game/BP_Board.BP_Board_C" (Math|Transform|MakeTransform "-1000000.000000,-1000000.000000,-100000.000000") "Undefined" "MultiplyWithRoot" 0 (LocalVariables|GetBag) 1e+01 true Probability 0))
    (Variables|Default|SetBoard _returnvalue_2)
    (else
      (bind _outactors (Actor|GetAllActorsOfClass "/Game/BP_Camera_Front.BP_Camera_Front_C"))
      (if (Utilities|Array|IsNotEmpty _outactors)
        (bind _returnvalue_3 (Game|SpawnActorfromClass "/Game/BP_Board.BP_Board_C" (Math|Conversions|ToTransform(Vector) (+ (Transformation|GetWorldLocation (Variables|/Game/BP_Camera_Front.BP_Camera_Front_C|GetCamera (Utilities|Array|Get(acopy) _outactors))) "0.000000,-189.000000,-100.000000")) "Undefined" "MultiplyWithRoot" 0 (LocalVariables|GetBag) 1e+01 false 0.1 0))
        (Variables|Default|SetBoard _returnvalue_3)))))

(fn GetWord
  (params (Tile%20Datas :type Array%20of%20Tile%20Data%20Structures))
  (for _array_element Tile%20Datas
    (LocalVariables|SetCurrent%20Word (Utilities|String|Append (LocalVariables|GetCurrent%20Word) (.letter _array_element))))
  (return (LocalVariables|GetCurrent%20Word)))

(fn ExecutePlayerAttack
  (bind _board (Variables|Default|GetBoard)
    (:then
      (bind (_is_valid _selected_tile_data) (CallFunction|CheckValidity))
      (if _is_valid
        (Variables|Default|SetCurrent%20Tile%20Data _selected_tile_data)
        (Default|RemoveSelectedTiles _board)
        (bind _asbp_turn_based_game_mode (Utilities|Casting|CastToBP_TurnBasedGameMode (Game|GetGameMode)))
        (CallFunction|MeleeAttack (Utilities|Array|Get(acopy) (Variables|/Game/BP_TurnBasedGameMode.BP_TurnBasedGameMode_C|GetEnemyUnits _asbp_turn_based_game_mode)))))
    (:else)))

(fn ClearBoard
  (bind _board (Variables|Default|GetBoard)
    (:then
      (Default|ClearBoard _board)
      (CallFunction|EndUnitTurn)
      ;[1 1 1] Disable action menu when executing action
      (bind _action_menu (Variables|Default|GetAction%20Menu)
        (:then
          (Widget|SetRenderOpacity _action_menu 0.5)
          (Widget|SetIsEnabled _action_menu false))
        (:else)))
    (:else)))

(fn CheckGameOver
  (params (CurrentPlayer :type BP%20Unit%20Base%20Object%20Reference))
  (return (<= (Variables|/Game/BP_UnitBase.BP_UnitBase_C|GetHealth_Current CurrentPlayer) 0.0) (== (Utilities|GetClass CurrentPlayer) "/Game/BP_TestEnemyUnit.BP_TestEnemyUnit_C")))

(fn UnselectTiles
  (Default|UnselectAll (Variables|Default|GetBoard)))

(fn Scramble
  (Default|ScrambleBoard (Variables|Default|GetBoard)))

(fn CheckValidity
  (bind _board (Variables|Default|GetBoard)
    (:then
      (bind _word (Default|GetSelectedTiles'Data _board))
      (bind _output_get (LocalVariables|SetTile%20Datas _word))
      (bind _word_2 (CallFunction|GetWord _output_get))
      (Development|PrintString _word_2)
      (bind _is_valid (CallFunction|CheckifWordIsValid _word_2))
      (return _is_valid (LocalVariables|GetTile%20Datas)))
    (:else)))