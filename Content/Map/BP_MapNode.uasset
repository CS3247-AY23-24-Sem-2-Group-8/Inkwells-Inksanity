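; BP_MapNode is a clickable node on the run map that opens a battle, rest, shop or boss level by icon type.
; Clicks only work on level-zero nodes at the start, then on unvisited nodes linked from the current node by GameInstance map edges.
; Battles randomize difficulty by node level, while bosses use fixed values.
; Selection saves visited state, current node and camera position to the GameInstance, and material swaps show hover and visited states.
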(event MouseInput|EventActorBeginCursorOver
  (if (not (Variables|Default|GetIs%20Visited))
    (Rendering|Material|SetMaterial (Variables|Default|GetStaticMesh) 0 (Utilities|Array|Get(acopy) (Variables|Default|GetPressedMaterialIcons) (Variables|Default|GetIcon%20Type)))))

(event MouseInput|EventActorOnClicked
  (params (ButtonPressed :type Key%20Structure))
  (bind _asbp_game_instance (Utilities|Casting|CastToBP_GameInstance (Game|GetGameInstance)))
  (if (Utilities|Operators|EqualEqual :A (Variables|/Game/BP_GameInstance.BP_GameInstance_C|GetCurrentNode _asbp_game_instance))
    (bind _returnvalue (Class|MapGeneration|GetNodeLevel (Math|Vector2D|MakeVector2D (.nodex (Utilities|Array|Get(acopy) (Variables|/Game/BP_GameInstance.BP_GameInstance_C|GetMap%20Nodes _asbp_game_instance) (Variables|Default|GetNodeIndex))) (.nodey (Utilities|Array|Get(acopy) (Variables|/Game/BP_GameInstance.BP_GameInstance_C|GetMap%20Nodes _asbp_game_instance) (Variables|Default|GetNodeIndex)))) (.height (Utilities|Array|Get(acopy) (Variables|/Game/BP_GameInstance.BP_GameInstance_C|GetMap%20Nodes _asbp_game_instance) (Variables|Default|GetNodeIndex))) (.heightscale (Utilities|Array|Get(acopy) (Variables|/Game/BP_GameInstance.BP_GameInstance_C|GetMap%20Nodes _asbp_game_instance) (Variables|Default|GetNodeIndex)))))
    (if (== _returnvalue 0)
      (switch int (Variables|Default|GetIcon%20Type) :!label _label
        (:Default
          (Development|PrintString "Unknown Node"))
        (:0
          (CallFunction|OnPressBattle _returnvalue)
          (bind _asbp_game_instance_2 (Utilities|Casting|CastToBP_GameInstance (Game|GetGameInstance) :!label _label_2))
          (|SetBy-RefVar (Utilities|Array|Get(acopy) (Variables|/Game/BP_GameInstance.BP_GameInstance_C|GetMap%20Nodes _asbp_game_instance_2) (Variables|Default|GetNodeIndex)) (Utilities|Struct|MakeMapNode (.MapX (Utilities|Struct|BreakMapNode (Utilities|Array|Get(acopy) (Variables|/Game/BP_GameInstance.BP_GameInstance_C|GetMap%20Nodes _asbp_game_instance_2) (Variables|Default|GetNodeIndex)))) (.MapY (Utilities|Struct|BreakMapNode (Utilities|Array|Get(acopy) (Variables|/Game/BP_GameInstance.BP_GameInstance_C|GetMap%20Nodes _asbp_game_instance_2) (Variables|Default|GetNodeIndex)))) (.IconType (Utilities|Struct|BreakMapNode (Utilities|Array|Get(acopy) (Variables|/Game/BP_GameInstance.BP_GameInstance_C|GetMap%20Nodes _asbp_game_instance_2) (Variables|Default|GetNodeIndex)))) true (.NodeX (Utilities|Struct|BreakMapNode (Utilities|Array|Get(acopy) (Variables|/Game/BP_GameInstance.BP_GameInstance_C|GetMap%20Nodes _asbp_game_instance_2) (Variables|Default|GetNodeIndex)))) (.NodeY (Utilities|Struct|BreakMapNode (Utilities|Array|Get(acopy) (Variables|/Game/BP_GameInstance.BP_GameInstance_C|GetMap%20Nodes _asbp_game_instance_2) (Variables|Default|GetNodeIndex)))) (.Height (Utilities|Struct|BreakMapNode (Utilities|Array|Get(acopy) (Variables|/Game/BP_GameInstance.BP_GameInstance_C|GetMap%20Nodes _asbp_game_instance_2) (Variables|Default|GetNodeIndex)))) (.HeightScale (Utilities|Struct|BreakMapNode (Utilities|Array|Get(acopy) (Variables|/Game/BP_GameInstance.BP_GameInstance_C|GetMap%20Nodes _asbp_game_instance_2) (Variables|Default|GetNodeIndex))))))
          (bind _asbp_game_instance_3 (Utilities|Casting|CastToBP_GameInstance (Game|GetGameInstance)))
          (Variables|/Game/BP_GameInstance.BP_GameInstance_C|SetCurrentNode _asbp_game_instance_3 (Math|Vector2D|MakeVector2D (.NodeX (Utilities|Struct|BreakMapNode (Utilities|Array|Get(acopy) (Variables|/Game/BP_GameInstance.BP_GameInstance_C|GetMap%20Nodes _asbp_game_instance_2) (Variables|Default|GetNodeIndex)))) (.NodeY (Utilities|Struct|BreakMapNode (Utilities|Array|Get(acopy) (Variables|/Game/BP_GameInstance.BP_GameInstance_C|GetMap%20Nodes _asbp_game_instance_2) (Variables|Default|GetNodeIndex))))))
          (Variables|Default|SetIs%20Visited true)
          (Rendering|Material|SetMaterial (Variables|Default|GetStaticMesh) 0 (Utilities|Array|Get(acopy) (Variables|Default|GetCancelledMaterialIcons) (Variables|Default|GetIcon%20Type)))
          (bind _returnvalue_2 (Actor|GetActorOfClass "/Script/Engine.CameraActor"))
          (Variables|/Game/BP_GameInstance.BP_GameInstance_C|SetCamera%20Position _asbp_game_instance_3 (Transformation|GetActorLocation _returnvalue_2)))
        (:1
          (CallFunction|OnPressRest)
          (goto _label_2))
        (:2
          (CallFunction|OnPressShop)
          (goto _label_2))
        (:3
          (CallFunction|OnPressBoss)
          (goto _label_2))))
    (elif (and (not (Variables|Default|GetIs%20Visited)) (Utilities|Array|ContainsItem (.To (Utilities|Struct|BreakMapEdgeList (.Value (Utilities|Map|Find (Variables|/Game/BP_GameInstance.BP_GameInstance_C|GetMapEdges _asbp_game_instance) (Variables|/Game/BP_GameInstance.BP_GameInstance_C|GetCurrentNode _asbp_game_instance))))) (Math|Vector|MakeVector (.nodex (Utilities|Array|Get(acopy) (Variables|/Game/BP_GameInstance.BP_GameInstance_C|GetMap%20Nodes _asbp_game_instance) (Variables|Default|GetNodeIndex))) (.nodey (Utilities|Array|Get(acopy) (Variables|/Game/BP_GameInstance.BP_GameInstance_C|GetMap%20Nodes _asbp_game_instance) (Variables|Default|GetNodeIndex))) 0.0)))
      (goto _label))))

(event MouseInput|EventActorEndCursorOver
  (if (not (Variables|Default|GetIs%20Visited))
    (Rendering|Material|SetMaterial (Variables|Default|GetStaticMesh) 0 (Utilities|Array|Get(acopy) (Variables|Default|GetMaterialInstances) (Variables|Default|GetIcon%20Type)))))

(fn ConstructionScript
  (if (Variables|Default|GetIs%20Visited)
    (Rendering|Material|SetMaterial (Variables|Default|GetStaticMesh) 0 (Utilities|Array|Get(acopy) (Variables|Default|GetCancelledMaterialIcons) (Variables|Default|GetIcon%20Type)))
    (else
      (Rendering|Material|SetMaterial (Variables|Default|GetStaticMesh) 0 (Utilities|Array|Get(acopy) (Variables|Default|GetMaterialInstances) (Variables|Default|GetIcon%20Type))))))

(fn OnPressRest
  (CameraFades|StartCameraFade :self (Game|GetPlayerCameraManager 0) :ToAlpha 1.0 :Duration 1.0 :bHoldWhenFinished true)
  (Game|OpenLevel(byName) "RestLevel"))

(fn OnPressShop
  (CameraFades|StartCameraFade :self (Game|GetPlayerCameraManager 0) :ToAlpha 1.0 :Duration 1.0 :bHoldWhenFinished true)
  (Game|OpenLevel(byName) "ShopLevel"))

(fn OnPressBoss
  (Development|PrintString "Pressed Boss Node")
  (bind _asbp_game_instance (Utilities|Casting|CastToBP_GameInstance (Game|GetGameInstance)))
  (Variables|/Game/BP_GameInstance.BP_GameInstance_C|SetMax%20Enemy%20Health _asbp_game_instance 1e+02)
  (Variables|/Game/BP_GameInstance.BP_GameInstance_C|SetLonger%20Word%20Probability _asbp_game_instance 0.8)
  (Variables|/Game/BP_GameInstance.BP_GameInstance_C|SetIsBossEncountered _asbp_game_instance true)
  (bind _returnvalue (Actor|GetActorOfClass "/Script/Engine.CameraActor"))
  (Variables|/Game/BP_GameInstance.BP_GameInstance_C|SetCamera%20Position _asbp_game_instance (Transformation|GetActorLocation _returnvalue))
  (CameraFades|StartCameraFade :self (Game|GetPlayerCameraManager 0) :ToAlpha 1.0 :Duration 1.0 :bHoldWhenFinished true)
  (Game|OpenLevel(byName) "TestBossLevel"))

(fn OnPressBattle
  (params (Node%20Level :type Integer))
  (bind _asbp_game_instance (Utilities|Casting|CastToBP_GameInstance (Game|GetGameInstance)))
  (Variables|/Game/BP_GameInstance.BP_GameInstance_C|SetMax%20Enemy%20Health _asbp_game_instance (Math|Random|RandomFloatinRange 2e+01 (+ 2e+01 (* (+ Node%20Level 1) 1e+01))))
  (Variables|/Game/BP_GameInstance.BP_GameInstance_C|SetLonger%20Word%20Probability _asbp_game_instance (Math|Random|RandomFloatinRange 0.0 (* 0.1 (+ Node%20Level 1))))
  (CameraFades|StartCameraFade :self (Game|GetPlayerCameraManager 0) :ToAlpha 1.0 :Duration 1.0 :bHoldWhenFinished true)
  (Game|OpenLevel(byName) (Utilities|String|StringToName (Utilities|Array|Get(acopy) (Variables|Default|GetLevelNames) (Math|Random|RandomIntegerinRange 0 1)))))