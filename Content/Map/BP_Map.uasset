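; BP_Map is a map actor that generates a three-path node graph across its own bounds on BeginPlay.
; GenerateCoordinates takes the actor's width and height and returns vertices plus edges stored as vertex index pairs.
; Each vertex is translated around the bounds origin to spawn a BP_MapNode.
; The edge loop is nested in the vertex loop, so every BP_Edge spawns again per vertex, receiving untranslated endpoints, origin and dimensions.
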(event EventBeginPlay
  (bind (_origin _boxextent) (Collision|GetActorBounds false false))
  (bind (_x _y) (Math|Vector|BreakVector _origin))
  (bind (_x_2 _y_2) (Math|Vector|BreakVector _boxextent))
  (Variables|Default|SetWidth (Math|Float|Truncate (* _x_2 2.0)))
  (Variables|Default|SetHeight (Math|Float|Truncate (* _y_2 2.0)))
  (bind (_vertices _edges) (Class|MapGeneration|GenerateCoordinates (Variables|Default|GetWidth) (Variables|Default|GetHeight) 3))
  (for _array_element _vertices
    (bind _returnvalue (Class|MapGeneration|TranslatetoMapCoordinates (Math|Vector2D|MakeVector2D (.x _array_element) (.y _array_element)) (Math|Vector2D|MakeVector2D _x _y) (Variables|Default|GetWidth) (Variables|Default|GetHeight)))
    (Game|SpawnActorfromClass "/Game/Map/BP_MapNode.BP_MapNode_C" (Math|Conversions|ToTransform(Vector) (Math|Vector|MakeVector (.x _returnvalue) (.y _returnvalue) 0.0)) "Undefined" "MultiplyWithRoot" 0 0)
    (for _array_element_2 _edges
      (Game|SpawnActorfromClass "/Game/Map/BP_Edge.BP_Edge_C" (Math|Transform|MakeTransform "0, 0, 0") "Undefined" "MultiplyWithRoot" 0 _origin (Math|Vector|MakeVector (.X (Math|Vector2D|BreakVector2D (Utilities|Array|Get(acopy) _vertices (Math|Float|Truncate (.X (Math|Vector2D|BreakVector2D _array_element_2)))))) (.Y (Math|Vector2D|BreakVector2D (Utilities|Array|Get(acopy) _vertices (Math|Float|Truncate (.X (Math|Vector2D|BreakVector2D _array_element_2)))))) 0.0) (Math|Vector|MakeVector (.X (Math|Vector2D|BreakVector2D (Utilities|Array|Get(acopy) _vertices (Math|Float|Truncate (.Y (Math|Vector2D|BreakVector2D _array_element_2)))))) (.Y (Math|Vector2D|BreakVector2D (Utilities|Array|Get(acopy) _vertices (Math|Float|Truncate (.Y (Math|Vector2D|BreakVector2D _array_element_2)))))) 0.0) (Variables|Default|GetWidth) (Variables|Default|GetHeight) 0))))

(fn ConstructionScript)