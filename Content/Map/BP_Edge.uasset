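; BP_Edge is a map actor that draws an edge between EdgeStart and EdgeEnd as a spline mesh, built in the construction script.
; Both endpoints get opposite Y nudges, go through TranslateToMapCoordinates using map origin and size, then set one segment at fixed height.
; The instanced mesh receives NewMesh but no instances.
; Spacing-based repetition via Pythagoras and per-spline-point segments are unconnected leftovers, and event graph nodes are disabled.
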(event EventBeginPlay)

(event Collision|EventActorBeginOverlap
  (params (OtherActor :type Actor%20Object%20Reference)))

(event EventTick
  (params (DeltaSeconds :type Float%20%28single-precision%29)))

(fn ConstructionScript
  (bind _edgestart (Variables|Default|GetEdgeStart))
  (bind _edgeend (Variables|Default|GetEdgeEnd))
  (bind _origin (Variables|Default|GetOrigin))
  (bind _width (Variables|Default|GetWidth))
  (bind _height (Variables|Default|GetHeight))
  (bind (_x _y) (Math|Vector|BreakVector _edgestart))
  (bind (_x_2 _y_2) (Math|Vector|BreakVector _edgeend))
  (bind (_x_3 _y_3) (Math|Vector|BreakVector _origin))
  (Components|StaticMesh|SetStaticMesh (Variables|Default|GetInstancedStaticMesh) (Variables|Default|GetNew%20Mesh))
  (bind _returnvalue (AddComponent|AddSplineMeshComponent false (Math|Transform|MakeTransform (Spline|GetLocationatDistanceAlongSpline (Variables|Default|GetSpline) (* (stale _index) (Variables|Default|GetSpacing)) "Local"))))
  ;[1 1 1] Edge Start Point
  (bind _returnvalue_2 (Class|MapGeneration|TranslatetoMapCoordinates (Math|Vector2D|MakeVector2D _x (+ _y 3e+01)) (Math|Vector2D|MakeVector2D _x_3 _y_3) _width _height 0.8 0.9))
  ;[1 1 1] Edge End Point
  (bind _returnvalue_3 (Class|MapGeneration|TranslatetoMapCoordinates (Math|Vector2D|MakeVector2D _x_2 (- _y_2 3e+01)) (Math|Vector2D|MakeVector2D _x_3 _y_3) _width _height 0.8 0.9))
  (SplineMesh|SetStartandEnd _returnvalue (Math|Conversions|ToVector(Vector2D) _returnvalue_2 1e+01) "0, 0, 0" (Math|Conversions|ToVector(Vector2D) _returnvalue_3 1e+01) "0, 0, 0" true :!class /Script/Engine.SplineMeshComponent))

(fn Pythagoras
  (params (Point1 :type Vector) (Point2 :type Vector))
  (bind (_x _y) (Math|Vector|BreakVector Point1))
  (bind (_x_2 _y_2) (Math|Vector|BreakVector Point2))
  (return (Math|Float|Sqrt (+ (Math|Float|Square (- _x _x_2)) (Math|Float|Square (- _y _y_2))))))