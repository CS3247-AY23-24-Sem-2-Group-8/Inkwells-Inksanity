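; BP_TestCharacterCamera is a test actor whose camera follows it along a spline rail.
; On BeginPlay it finds and caches the BP_CameraSpline actor in the level.
; Each tick it finds the spline point closest to its own location and eases the camera's world position toward it with VInterpTo.
; Only the camera's location is driven here; its rotation is untouched.
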(event EventBeginPlay
  (bind _returnvalue (Actor|GetActorOfClass "/Game/BP_CameraSpline.BP_CameraSpline_C"))
  (Variables|Default|SetCamera%20Spline%20REF _returnvalue))

(event EventTick
  (params (DeltaSeconds :type Float%20%28single-precision%29))
  ;[1 1 1] Move Camera
  (Transformation|SetWorldLocation (Variables|Default|GetCamera) (Math|Interpolation|VInterpTo (Transformation|GetWorldLocation (Variables|Default|GetCamera)) (Spline|FindLocationClosesttoWorldLocation (Variables|/Game/BP_CameraSpline.BP_CameraSpline_C|GetSpline (Variables|Default|GetCamera%20Spline%20REF)) (Transformation|GetActorLocation) "World") (Utilities|Time|GetWorldDeltaSeconds) 2.0) false false))

(fn ConstructionScript)