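; BP_Tile is a clickable letter tile actor for what appears to be a board-based word game.
; On BeginPlay, it passes the letter from its TileData to a BP_Tile_Word widget on its widget component.
; Clicking the cube, when a Board reference is valid, notifies the board before toggling IsSelected.
; SetHighlighted then shows or hides the Highlight component and its children to match the selection.
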(event OnClicked(Cube)
  (params (TouchedComponent :type Primitive%20Component%20Object%20Reference) (ButtonPressed :type Key%20Structure :default "None"))
  (bind _board (Variables|Default|GetBoard)
    (:then
      (Default|OnTileSelected _board self)
      (if (Variables|Default|GetIs%20Selected)
        (Variables|Default|SetIs%20Selected false)
        (else
          (Variables|Default|SetIs%20Selected true)))
      (CallFunction|SetHighlighted (Variables|Default|GetIs%20Selected)))
    (:else)))

(event EventBeginPlay
  (bind _asbp_tile_word (Utilities|Casting|CastToBP_Tile_Word (UserInterface|GetUserWidgetObject (Variables|Default|GetWidget))))
  (Default|SetLetter _asbp_tile_word (Utilities|Text|ToText(String) (.letter (Variables|Default|GetTile%20Data)))))

(event Collision|EventActorBeginOverlap
  (params (OtherActor :type Actor%20Object%20Reference)))

(event EventTick
  (params (DeltaSeconds :type Float%20%28single-precision%29)))

(fn ConstructionScript)

(fn SetHighlighted
  (params (Is%20Highlighted :type Boolean))
  (Rendering|SetVisibility (Variables|Default|GetHighlight) Is%20Highlighted true))